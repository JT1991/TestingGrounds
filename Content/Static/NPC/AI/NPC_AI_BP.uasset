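; NPC_AI_BP is an AI controller for guard NPCs that starts their behavior tree and reports perceived targets to it.
; On BeginPlay it sets up the PatrolData blackboard and runs the GuardBehaviour tree.
; AI perception updates store any sensed actor without the "Guard" tag under the blackboard's enemy key, and clear that key when such an actor is no longer sensed.
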(event OnTargetPerceptionUpdated(AIPerception)
  (params (Actor :type Actor%20Object%20Reference) (Stimulus :type AI%20Stimulus%20Structure))
  (bind _enemykey (Variables|Default|GetEnemyKey))
  (bind _blackboardcomp (Variables|Default|GetBlackboardComp))
  (if (not (Actor|ActorHasTag Actor "Guard"))
    (if (.bSuccessfullySensed (Utilities|Struct|BreakAIStimulus Stimulus))
      (AI|Components|Blackboard|SetValueasObject _blackboardcomp _enemykey Actor)
      (else
        (AI|Components|Blackboard|ClearValue _blackboardcomp _enemykey)))))

(event EventBeginPlay
  (bind _blackboardcomponent (Class|AIController|UseBlackboard "/Game/Static/NPC/AI/PatrolData.PatrolData"))
  (AI|RunBehaviorTree "/Game/Static/NPC/AI/GuardBehaviour.GuardBehaviour")
  (Variables|Default|SetBlackboardComp _blackboardcomponent))

(event EventTick
  (params (DeltaSeconds :type Float%20%28single-precision%29)))

(fn ConstructionScript)