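; BP_Tile is an infinite-terrain tile that scatters containers, boxes and rocks on BeginPlay through PlaceActors calls.
; Its barrier starts red and solid, turning green and passable while the player overlaps the locking volume.
; Player overlap with the destroy volume asks InfiniteTerrainGameMode to spawn a tile, then destroys this one; a hit only destroys it.
; An arrow component supplies the tile's attach transform.
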(event OnComponentBeginOverlap(LockingVolume)
  (params (OverlappedComponent :type Primitive%20Component%20Object%20Reference) (OtherActor :type Actor%20Object%20Reference) (OtherComp :type Primitive%20Component%20Object%20Reference) (OtherBodyIndex :type Integer) (bFromSweep :type Boolean) (SweepResult :type Hit%20Result%20Structure%20%28by%20ref%29))
  (Utilities|IsPlayerActor OtherActor)
  (CallFunction|UnlockLevel))

(event OnComponentEndOverlap(LockingVolume)
  (params (OverlappedComponent :type Primitive%20Component%20Object%20Reference) (OtherActor :type Actor%20Object%20Reference) (OtherComp :type Primitive%20Component%20Object%20Reference) (OtherBodyIndex :type Integer))
  (Utilities|IsPlayerActor OtherActor)
  (CallFunction|Lock))

(event OnComponentHit(DestroyTileVolume)
  (params (HitComponent :type Primitive%20Component%20Object%20Reference) (OtherActor :type Actor%20Object%20Reference) (OtherComp :type Primitive%20Component%20Object%20Reference) (NormalImpulse :type Vector :default "0, 0, 0") (Hit :type Hit%20Result%20Structure%20%28by%20ref%29))
  (Utilities|IsPlayerActor OtherActor)
  (Actor|DestroyActor))

(event OnComponentBeginOverlap(DestroyTileVolume)
  (params (OverlappedComponent :type Primitive%20Component%20Object%20Reference) (OtherActor :type Actor%20Object%20Reference) (OtherComp :type Primitive%20Component%20Object%20Reference) (OtherBodyIndex :type Integer) (bFromSweep :type Boolean) (SweepResult :type Hit%20Result%20Structure%20%28by%20ref%29))
  (Utilities|IsPlayerActor OtherActor)
  (bind _asinfinite_terrain_game_mode (Utilities|Casting|CastToInfiniteTerrainGameMode (Game|GetGameMode)))
  (Default|SpawnTIle _asinfinite_terrain_game_mode)
  (Actor|DestroyActor))

(event EventBeginPlay
  (CallFunction|Lock)
  (Class|Tile|PlaceActors "/Game/Dynamic/Terrain/Props/BP_Container.BP_Container_C" 1 3 4e+02 1.0 1.0)
  (Class|Tile|PlaceActors "/Game/Dynamic/Terrain/Props/BP_Cannister.BP_Cannister_C" 0 0 5e+01 1.0 1.0)
  (Class|Tile|PlaceActors "/Game/Dynamic/Terrain/Props/BP_Box.BP_Box_C" 2 4 1e+02 1.0 1.0)
  (Class|Tile|PlaceActors "/Game/Dynamic/Terrain/Props/BP_Rock01.BP_Rock01_C" 2 8 1.5e+02 1.0 5.0)
  (Class|Tile|PlaceActors "/Game/BP_Rock05.BP_Rock05_C" 1 3 2.5e+02 1.0 1.0)
  (Class|Tile|PlaceActors "/Game/BP_Rock17.BP_Rock17_C" 0 1 2.5e+02 1.0 1.0))

(fn ConstructionScript)

(fn GetAttachLocation
  (return (Transformation|GetWorldTransform (Variables|Default|GetArrow))))

(fn UnlockLevel
  (Collision|SetCollisionEnabled (Variables|Default|GetBarrier) "NoCollision")
  (Rendering|Material|SetMaterial (Variables|Default|GetBarrier) 0 "/Game/Dynamic/Terrain/MI_Barrier_Green.MI_Barrier_Green"))

(fn Lock
  (Collision|SetCollisionEnabled (Variables|Default|GetBarrier) "QueryAndPhysics")
  (Rendering|Material|SetMaterial (Variables|Default|GetBarrier) 0 "/Game/Dynamic/Terrain/MI_Barrier_Red.MI_Barrier_Red"))