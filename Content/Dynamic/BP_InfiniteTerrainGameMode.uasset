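; Game mode for an infinite terrain level that spawns the terrain tiles and keeps the score.
; On BeginPlay it populates a pool of NavMesh bounds volumes, then spawns an initial run of tiles.
; Each spawned BP_Tile receives the shared volume pool and supplies its attach location as the next tile's transform, chaining the terrain end to end.
; Score increments through NewTIleConquered and is exposed through GetScore.
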(event EventBeginPlay
  (Class|InfiniteTerrainGameMode|PopulateBoundsVoumePool)
  (for _index (range 0 3)
    (CallFunction|SpawnTIle)))

(fn ConstructionScript)

(fn SpawnTIle
  (bind _returnvalue (Game|SpawnActorfromClass "/Game/Dynamic/Terrain/BP_Tile.BP_Tile_C" (Variables|Default|GetNextTileTransform) "Undefined" 0 0))
  (Class|Tile|SetPool _returnvalue (Variables|Default|GetNavMeshBoundsVolumePool))
  (bind _attach_transform (Default|GetAttachLocation _returnvalue))
  (Variables|Default|SetNextTileTransform _attach_transform))

(fn NewTIleConquered
  (Math|Integer|IncrementInt (Variables|Default|GetScore)))

(fn GetScore
  (return (Variables|Default|GetScore)))